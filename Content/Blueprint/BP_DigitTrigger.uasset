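; BP_DigitTrigger is an interactable trigger that responds to CanInteract interface events.
; Widget requests add a BP_CanInteract widget to the viewport, and closing clears all widgets rather than just that one.
; Interact requests disable and re-enable the trigger's own input for the first player controller.
; The NumberDigit event is unused, and the file shows no digit logic.
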(event OpenRequestWidget(CanInteract)
  (bind _returnvalue (UserInterface|CreateWidget "/Game/UI/BP_CanInteract.BP_CanInteract_C" (Game|GetPlayerController 0)))
  (UserInterface|Viewport|AddtoViewport _returnvalue 0))

(event CloseRequestWidget(CanInteract)
  (Viewport|RemoveAllWidgets))

(event OpenRequestInteract(CanInteract)
  (Input|DisableInput (Game|GetPlayerController 0)))

(event CloseRequestInteract(CanInteract)
  (Input|EnableInput (Game|GetPlayerController 0)))

(fn ConstructionScript)